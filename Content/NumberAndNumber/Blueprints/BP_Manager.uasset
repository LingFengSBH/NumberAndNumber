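; Manager actor for a click-based number-card matching game, where three identical numbers in the slot list clear.
; Initialize, run on construction and BeginPlay, gives random triples of BP_NumberCard actors a shared random number, so numbers come in threes.
; Add appends a number, removes matched triples with a sound, then rebuilds the row of TextRender components showing the list.
; Adding to a full list prints a death message and pauses the game.
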(event `self.ReceiveBeginPlay`
  (bind _returnvalue (`GameplayStatics.GetPlayerController` 0))
  (`self.Initialize`)
  (`GameplayStatics.PlaySound2D` "/Game/StarterContent/Audio/Starter_Music01.Starter_Music01" 1.0 1.0 0.0 null null)
  ;[1 1 1] 使用点击事件来交互Card
  (set `PlayerController.bShowMouseCursor` true _returnvalue)
  (set `PlayerController.bEnableClickEvents` true _returnvalue))

(event `Add`
  (params (NewItem :type "Integer (by ref)"))
  (bind _textarray (`self.TextArray`))
  (set `self.NewItem` NewItem)
  (if (>= (`KismetArrayLibrary.Array_Length` (`self.Array`)) 10)
    ;[1 1 1] 槽位满了
    (`KismetSystemLibrary.PrintString` "你死了")
    (`GameplayStatics.SetGamePaused` true)
    (else
      (`KismetArrayLibrary.Array_Add` (`self.Array`) (`self.NewItem`))
      (set `self.Accu` 0)
      (for _array_element (`self.Array`)
        ;[1 1 1] 累加判断同样数字数量
        (if (== _array_element (`self.NewItem`))
          (`/Engine/EditorBlueprintResources/StandardMacros.IncrementInt` (`self.Accu`))))
      (if (>= (`self.Accu`) 3)
        ;[1 1 1] 移除所有的相同的数
        (`KismetArrayLibrary.Array_RemoveItem` (`self.Array`) (`self.NewItem`))
        (`GameplayStatics.PlaySound2D` "/Engine/EditorSounds/GamePreview/PossessPlayer.PossessPlayer" 1.0 1.0 0.0 null null))
      (for _array_element_2 _textarray
        ;[1 1 1] 清除所有TextRender再刷新新的
        (`ActorComponent.K2_DestroyComponent` _array_element_2))
      (`KismetArrayLibrary.Array_Clear` _textarray)
      (for (_array_element_3 _array_index) (`self.Array`)
        ;[1 1 1] 生成一串新的Text
        (bind _returnvalue (`AddComponent|NODE_AddTextRenderComponent-0` :`RelativeTransform` (`KismetMathLibrary.MakeTransform` (`KismetMathLibrary.MakeVector` 0.0 (`KismetMathLibrary.Conv_IntToDouble` (* _array_index 100)) 1.0) (struct :`Pitch` 90.0 :`Yaw` 180.0))))
        (`TextRenderComponent.K2_SetText` _returnvalue (`KismetTextLibrary.Conv_IntToText` _array_element_3))
        (`KismetArrayLibrary.Array_Add` (`self.TextArray`) _returnvalue)))))

(fn `Initialize`
  (bind _outactors (`GameplayStatics.GetAllActorsOfClass` "/Game/NumberAndNumber/Blueprints/BP_NumberCard.BP_NumberCard_C"))
  (bind _output_get (set `self.Out Actors` _outactors))
  (set `self.LastLoopIndex` (- (/ (`KismetArrayLibrary.Array_Length` _output_get) 3) 1))
  (for _ (range (+ (`self.LastLoopIndex`) 1))
    (set `self.Random` (`KismetMathLibrary.RandomInteger` 7))
    (for _ (range 3)
      (bind _output_get_2 (set `self.TheCard` (`KismetArrayLibrary.Array_Random` (`self.Out Actors`))))
      (`/Game/NumberAndNumber/Blueprints/BP_NumberCard.SetNum` _output_get_2 (`self.Random`))
      (`KismetArrayLibrary.Array_RemoveItem` (`self.Out Actors`) _output_get_2))))

(fn `UserConstructionScript`
  (`self.Initialize`))