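; BP_NumberCard is a clickable numbered card for a stacked-tile game, selectable only when no card lies on top.
; Cover box-overlaps the space above on a 50 cm grid to set the covered state and number colour.
; A blocked click only gives feedback; a free click sends its number to BP_Manager and destroys the card.
; Before destruction it disables collision so cards below can correctly recheck their cover.
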(event `self.ReceiveBeginPlay`
  (`self.Cover`))

(event `self.Plane.OnClicked`
  (params (TouchedComponent :type "PrimitiveComponent Object Reference") (ButtonPressed :type "Key Structure"))
  (if (`self.Covered`)
    (`KismetSystemLibrary.PrintString` "挡住了")
    (`GameplayStatics.PlaySound2D` "/Engine/VREditor/Sounds/UI/Camera_Shutter.Camera_Shutter" 1.0 1.0 0.0 null null)
    (else
      (`self.Remove`)
      (`GameplayStatics.PlaySound2D` "/Engine/VREditor/Sounds/UI/Click_on_Button.Click_on_Button" 1.0 1.0 0.0 null null)
      (`self.K2_DestroyActor`))))

(event `CoverRemove`
  (`self.Cover`))

(fn `Cover`
  (returns (ReturnValue :type Boolean))
  ;[1 1 1] 坐标50cm对齐，所以这样检测
  ;;[1 1 1] 顶上有没有Card
  (bind (_outactors _returnvalue) (`KismetSystemLibrary.BoxOverlapActors` (+ (`self.K2_GetActorLocation`) (0.0 0.0 50.0)) (40.0 40.0 20.0) (`|MakeArray` "ObjectTypeQuery2" :!type "EObjectTypeQuery Enum") "BP_NumberCard_C"))
  (bind _output_get (set `self.Covered` _returnvalue))
  (`TextRenderComponent.SetTextRenderColor` (`self.TextRender`) (select `bool` _output_get :`false` (make `Color` 0 0 0 255) :`true` (make `Color` 0 0 255 255) :!type "Color Structure"))
  (return _output_get))

(fn `Remove`
  ;[1 1 1] 告诉Manager自己被点了
  (bind _returnvalue (`GameplayStatics.GetActorOfClass` "/Game/NumberAndNumber/Blueprints/BP_Manager.BP_Manager_C"))
  (`/Game/NumberAndNumber/Blueprints/BP_Manager.Add` _returnvalue (`self.Index`))
  ;[1 1 1] 防止被重复检测到底下的Card以为仍然被覆盖
  (`PrimitiveComponent.SetCollisionEnabled` (`self.Plane`) "NoCollision")
  ;[1 1 1] 检测底下的Card
  (bind _outactors (`KismetSystemLibrary.BoxOverlapActors` (+ (`self.K2_GetActorLocation`) (0.0 0.0 -50.0)) (40.0 40.0 20.0) (`|MakeArray` "ObjectTypeQuery2" :!type "EObjectTypeQuery Enum") "BP_NumberCard_C"))
  (for _array_element _outactors
    (bind _asbp_number_card (cast `/Game/NumberAndNumber/Blueprints/BP_NumberCard` _array_element))
    (`self.CoverRemove` _asbp_number_card)))

(fn `SetNum`
  (params (Index :type Integer))
  (bind _output_get (set `self.Index` Index))
  (`TextRenderComponent.K2_SetText` (`self.TextRender`) (`KismetTextLibrary.Conv_IntToText` _output_get)))

(fn `UserConstructionScript`)